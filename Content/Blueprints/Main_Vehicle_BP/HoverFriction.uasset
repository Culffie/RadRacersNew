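; Player hover racing vehicle that rides track surfaces and can latch overlapping AI vehicles to either side with F ("friction").
; Tick, enabled by StartHover, interpolates throttle-driven speed and sphere-traces downward to align to the surface normal, falling when nothing is hit.
; Holding Enter switches off gravity for free pitch/roll flight; zero health briefly hides the craft, then restores it.
; Boost, overheat, damage-collision and stuck-respawn logic is unwired; Space is a damage test.
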(event `CustomEvent_0`
  (`|ExecutionSequence`
    (:`then_0`
      (`/Engine/EditorBlueprintResources/StandardMacros.IsValid` (`self.BoostTrail`)
        (:`Is Valid`
          (bind _returnvalue (`GameplayStatics.SpawnEmitterAtLocation` "/Game/Art/Particles/Par_Thrust.Par_Thrust" (`SceneComponent.K2_GetComponentLocation` (`self.BoostTrail`))))
          (set `self.ParticleSystem` _returnvalue))))))

(event `self.FricCollR.OnComponentBeginOverlap`
  (params (OverlappedComponent :type "PrimitiveComponent Object Reference") (OtherActor :type "Actor Object Reference") (OtherComp :type "PrimitiveComponent Object Reference") (OtherBodyIndex :type Integer) (bFromSweep :type Boolean) (SweepResult :type "HitResult Structure (by ref)"))
  ;[1 1 1] Friction
  (bind _asai (cast `/Game/Blueprints/AI_BP/AI` OtherActor))
  (if (`PrimitiveComponent.IsOverlappingComponent` (`self.FricCollR`) (`/Game/Blueprints/AI_BP/AI.fricCollAiL` _asai))
    (set `self.FrictionOverlap` true)
    (set `self.FricR` true)
    (`KismetSystemLibrary.PrintString` "Overlap Right")
    (else
      (set `self.FrictionOverlap` false))))

(event `self.HealthColl.OnComponentBeginOverlap`
  (params (OverlappedComponent :type "PrimitiveComponent Object Reference") (OtherActor :type "Actor Object Reference") (OtherComp :type "PrimitiveComponent Object Reference") (OtherBodyIndex :type Integer) (bFromSweep :type Boolean) (SweepResult :type "HitResult Structure (by ref)"))
  ;[1 1 1] Damage & Health
)

(event `self.DamageColl.OnComponentBeginOverlap`
  (params (OverlappedComponent :type "PrimitiveComponent Object Reference") (OtherActor :type "Actor Object Reference") (OtherComp :type "PrimitiveComponent Object Reference") (OtherBodyIndex :type Integer) (bFromSweep :type Boolean) (SweepResult :type "HitResult Structure (by ref)"))
  ;[1 1 1] Damage & Health
)

(event `self.WallColl.OnComponentBeginOverlap`
  (params (OverlappedComponent :type "PrimitiveComponent Object Reference") (OtherActor :type "Actor Object Reference") (OtherComp :type "PrimitiveComponent Object Reference") (OtherBodyIndex :type Integer) (bFromSweep :type Boolean) (SweepResult :type "HitResult Structure (by ref)"))
  ;[1 1 1] Damage & Health
)

(event `Key|F`
  (params (Key :type "Key Structure"))
  ;[1 1 1] Friction
  (:`Pressed`
    (if (`self.FricR`)
      (if (`self.IsFricPlayer`)
        (set `self.CurrentSpeed` (`self.CurrentSpeed`))
        (set `self.IsFricPlayer` false)
        (set `self.PlayerInput` true)
        (bind _returnvalue (`SceneComponent.GetAttachParent` (`/Game/Blueprints/AI_BP/AI.fricCollAiL` (stale `self.FricCollR.OnComponentBeginOverlap` _asai))))
        (`SceneComponent.K2_DetachFromComponent` _returnvalue "KeepWorld" "KeepWorld" "KeepWorld" false)
        (elif (`self.FrictionOverlap`)
          (set `self.IsFricPlayer` true)
          (set `self.PlayerInput` false)
          (set `self.CurrentSpeed` (`KismetMathLibrary.FClamp` 0.0 0.0 200.0))
          (`SceneComponent.K2_AttachToComponent` _returnvalue (`self.FricSpringR`) "None" "SnapToTarget" "SnapToTarget" "KeepWorld" true)))
      (elif (`self.FricL`)
        (if (`self.IsFricPlayer`)
          (set `self.CurrentSpeed` (`self.CurrentSpeed`))
          (set `self.IsFricPlayer` false)
          (set `self.PlayerInput` true)
          (bind _returnvalue_2 (`SceneComponent.GetAttachParent` (`/Game/Blueprints/AI_BP/AI.fricCollAiR` (stale `self.FricCollL.OnComponentBeginOverlap` _asai))))
          (`SceneComponent.K2_DetachFromComponent` _returnvalue_2 "KeepWorld" "KeepWorld" "KeepWorld" false)
          (elif (`self.FrictionOverlap`)
            (set `self.IsFricPlayer` true)
            (set `self.PlayerInput` false)
            (set `self.CurrentSpeed` (`KismetMathLibrary.FClamp` 0.0 0.0 200.0))
            (`SceneComponent.K2_AttachToComponent` _returnvalue_2 (`self.FricSpringL`) "None" "SnapToTarget" "SnapToTarget" "KeepWorld" true)))))))

(event `self.FricCollL.OnComponentBeginOverlap`
  (params (OverlappedComponent :type "PrimitiveComponent Object Reference") (OtherActor :type "Actor Object Reference") (OtherComp :type "PrimitiveComponent Object Reference") (OtherBodyIndex :type Integer) (bFromSweep :type Boolean) (SweepResult :type "HitResult Structure (by ref)"))
  ;[1 1 1] Friction
  (bind _asai (cast `/Game/Blueprints/AI_BP/AI` OtherActor))
  (if (`PrimitiveComponent.IsOverlappingComponent` (`self.FricCollL`) (`/Game/Blueprints/AI_BP/AI.fricCollAiR` _asai))
    (set `self.FrictionOverlap` true)
    (set `self.FricL` true)
    (`KismetSystemLibrary.PrintString` "Overlap Left")
    (else
      (set `self.FrictionOverlap` false))))

(event `self.GravColl.OnComponentBeginOverlap`
  (params (OverlappedComponent :type "PrimitiveComponent Object Reference") (OtherActor :type "Actor Object Reference") (OtherComp :type "PrimitiveComponent Object Reference") (OtherBodyIndex :type Integer) (bFromSweep :type Boolean) (SweepResult :type "HitResult Structure (by ref)"))
  ;[1 1 1] Gravity Toggle
)

(event `Key|SpaceBar`
  (params (Key :type "Key Structure"))
  (bind _health (`self.Health`))
  ;[1 1 1] Health Test
  (:`Pressed`
    (if (> _health 0)
      (bind _output_get (set `self.Health` (- _health 10)))
      (`KismetSystemLibrary.PrintString` (`KismetStringLibrary.Conv_IntToString` _output_get) true true (struct :`R` 0.305375 :`G` 1.0 :`B` 0.040415 :`A` 1.0))
      (else
        (`KismetSystemLibrary.PrintString` "Dead")))))

(event `Key|Enter`
  (params (Key :type "Key Structure"))
  (bind _cube (`self.Cube`))
  ;[1 1 1] Gravity Toggle
  (:`Pressed`
    (set `self.Gravity` false)
    (`KismetSystemLibrary.PrintString` "Gravity Off")
    (`PrimitiveComponent.SetSimulatePhysics` _cube true)
    (`PrimitiveComponent.SetEnableGravity` _cube false))
  (:`Released`
    (set `self.Gravity` true)
    (`KismetSystemLibrary.PrintString` "Gravity On")
    (`PrimitiveComponent.SetSimulatePhysics` _cube false)))

(event `self.GravColl.OnComponentEndOverlap`
  (params (OverlappedComponent :type "PrimitiveComponent Object Reference") (OtherActor :type "Actor Object Reference") (OtherComp :type "PrimitiveComponent Object Reference") (OtherBodyIndex :type Integer))
  ;[1 1 1] Gravity Toggle
)

(event `self.FricCollR.OnComponentEndOverlap`
  (params (OverlappedComponent :type "PrimitiveComponent Object Reference") (OtherActor :type "Actor Object Reference") (OtherComp :type "PrimitiveComponent Object Reference") (OtherBodyIndex :type Integer))
  ;[1 1 1] Friction
  (bind _asai (cast `/Game/Blueprints/AI_BP/AI` OtherActor))
  (if (`PrimitiveComponent.IsOverlappingComponent` (`self.FricCollR`) (`/Game/Blueprints/AI_BP/AI.fricCollAiL` _asai))
    (set `self.FrictionOverlap` true)
    (else
      (set `self.FrictionOverlap` false)
      (set `self.FricR` false))))

(event `self.ReceiveBeginPlay`
  (`self.SetActorTickEnabled` false)
  ;[1 1 1] Countdown Interface
  (bind _asmy_player_controller (cast `/Game/Blueprints/My_Player_Controller_BP/MyPlayerController` (`GameplayStatics.GetPlayerController` 0)))
  (bind _output_get (set `self.ControllerReference` _asmy_player_controller))
  (set `/Game/Blueprints/My_Player_Controller_BP/MyPlayerController.RespawnLocation` (`self.GetTransform`) _output_get)
  (set `self.Health` 100))

(event `self.FricCollL.OnComponentEndOverlap`
  (params (OverlappedComponent :type "PrimitiveComponent Object Reference") (OtherActor :type "Actor Object Reference") (OtherComp :type "PrimitiveComponent Object Reference") (OtherBodyIndex :type Integer))
  ;[1 1 1] Friction
  (bind _asai (cast `/Game/Blueprints/AI_BP/AI` OtherActor))
  (if (`PrimitiveComponent.IsOverlappingComponent` (`self.FricCollL`) (`/Game/Blueprints/AI_BP/AI.fricCollAiR` _asai))
    (set `self.FrictionOverlap` true)
    (else
      (set `self.FrictionOverlap` false)
      (set `self.FricL` false))))

(event `/Game/Blueprints/Main_Vehicle_BP/HoverInterface.StartHover`
  ;[1 1 1] Countdown Interface
  (`self.SetActorTickEnabled` true))

(event `InputAxis|Throttle/ Pitch`
  (params (AxisValue :type "Float (single-precision)"))
  ;[1 1 1] Zero G Flight
  (if (not (`self.Gravity`))
    (`self.K2_AddActorLocalRotation` (`KismetMathLibrary.MakeRotator` 0.0 (`KismetMathLibrary.FClamp` (`KismetMathLibrary.FInterpTo` AxisValue 10.0 (`GameplayStatics.GetWorldDeltaSeconds`) 0.5) 0.0 5.0)))))

(event `InputAxis|Yaw`
  (params (AxisValue :type "Float (single-precision)"))
  ;[1 1 1] Zero G Flight
  (if (not (`self.Gravity`))
    (`self.K2_AddActorLocalRotation` (`KismetMathLibrary.MakeRotator` (`KismetMathLibrary.FInterpTo` AxisValue 10.0 (`GameplayStatics.GetWorldDeltaSeconds`) 0.5)))))

(event `self.ReceiveTick`
  (params (DeltaSeconds :type "Float (single-precision)"))
  (bind _cube (`self.Cube`))
  (bind _cube_2 (`self.Cube`))
  ;[1 1 1] Tick - Move Forward/Backward
  (`|ExecutionSequence`
    (:`then_0`
      (if (`self.Gravity`)
        (bind _output_get (set `self.CurrentSpeed` (`KismetMathLibrary.FInterpTo` (`self.CurrentSpeed`) (`self.DesiredSpeed`) (`GameplayStatics.GetWorldDeltaSeconds`) (/ (`self.AccelerationInterp`) 2.0))))
        (`self.K2_AddActorLocalOffset` (`KismetMathLibrary.MakeVector` _output_get) true)
        (`self.Line trace safety`)
        ;[1 1 1] Death & Respawn
        (if (<= (`self.Health`) 0)
          (`self.DisableInput` null)
          (`PrimitiveComponent.SetCollisionEnabled` _cube_2 "NoCollision")
          (`SceneComponent.SetVisibility` _cube_2 false false)
          (set `self.DesiredSpeed` 0.0)
          (set `self.CurrentSpeed` 0.0)
          (`KismetSystemLibrary.Delay` 2.0)
          (set `self.Health` 100)
          (`self.EnableInput` null)
          (`SceneComponent.SetVisibility` _cube true false)
          (`KismetSystemLibrary.Delay` 2.0)
          (`PrimitiveComponent.SetCollisionEnabled` _cube "QueryAndPhysics"))
        (else
          (bind _output_get_2 (set `self.CurrentSpeed` (`self.CurrentSpeed`)))
          (`self.K2_AddActorLocalOffset` (`KismetMathLibrary.MakeVector` _output_get_2) true)
          (`self.Line trace safety`))))))

(event `Key|LeftShift`
  (params (Key :type "Key Structure"))
  ;[1 1 1] Boost
  (:`Pressed`
    (if (<= (`self.Boost`) 0.0)
      (`KismetSystemLibrary.PrintString` "BOOST OUT")
      (elif (`self.Overheated`)
        (`KismetSystemLibrary.PrintString` "OVERHEATED" true true (struct :`R` 0.233333 :`G` 0.074144 :`B` 0.021562 :`A` 1.0))
        (else
          (set `self.BoostActive` true)))))
  (:`Released`
    (set `self.BoostActive` false)))

(event `Key|W`
  (params (Key :type "Key Structure"))
  ;[1 1 1] Zero G Flight
  (:`Pressed`
    (set `self.ControlFlight` true))
  (:`Released`
    (set `self.ControlFlight` false)))

(event `self.ReceiveDestroyed`
  (`/Game/Blueprints/My_Player_Controller_BP/MyPlayerController.RespawnVehicle` (`self.ControllerReference`)))

(event `InputAxis|Throttle/ Pitch`
  (params (AxisValue :type "Float (single-precision)"))
  ;[1 1 1] Throttle
  (if (`self.Gravity`)
    (if (> AxisValue 0.0)
      (set `self.DesiredSpeed` (`KismetMathLibrary.FInterpTo` (`self.DesiredSpeed`) (`self.MaxSpeed`) (`GameplayStatics.GetWorldDeltaSeconds`) (`self.AccelerationInterp`)))
      (elif (< AxisValue 0.0)
        (set `self.DesiredSpeed` (`KismetMathLibrary.FInterpTo` (`self.DesiredSpeed`) (* (/ (`self.MaxSpeed`) 2.0) -1.0) (`GameplayStatics.GetWorldDeltaSeconds`) (`self.AccelerationInterp`)))
        (elif (== 0.0 0.0)
          (set `self.DesiredSpeed` (`KismetMathLibrary.FInterpTo` (`self.DesiredSpeed`) 0.0 (`GameplayStatics.GetWorldDeltaSeconds`))))))))

(event `self.BoostColl.OnComponentBeginOverlap`
  (params (OverlappedComponent :type "PrimitiveComponent Object Reference") (OtherActor :type "Actor Object Reference") (OtherComp :type "PrimitiveComponent Object Reference") (OtherBodyIndex :type Integer) (bFromSweep :type Boolean) (SweepResult :type "HitResult Structure (by ref)"))
  ;[1 1 1] Boostpads
  (cast `/Game/Blueprints/Power_Up_BP/BoostPad` OtherActor)
  (`KismetSystemLibrary.PrintString` "Boost Hit")
  (set `self.BoostPad` true)
  (`KismetSystemLibrary.Delay` 2.0)
  (set `self.BoostPad` false))

(event `Start Camera Location`
  (bind (_returnvalue_x _returnvalue_y _returnvalue_z) (`KismetMathLibrary.BreakVector` (`KismetMathLibrary.Normal` (`self.deltaS`))))
  (bind (_returnvalue_roll _returnvalue_pitch _returnvalue_yaw) (`KismetMathLibrary.BreakRotator` (`KismetMathLibrary.InverseTransformRotation` (`self.GetTransform`) (`KismetMathLibrary.FindLookAtRotation` (0.0 0.0 0.0) (/ (+ (`KismetMathLibrary.MakeVector` (* _returnvalue_x 100.0) (* _returnvalue_y 100.0) (* _returnvalue_z 200.0)) (* (`SceneComponent.GetForwardVector` (`self.Cube`)) 4.0)) 1.0)))))
  ;[1 1 1] Camera Location
  (`SceneComponent.K2_SetRelativeLocation` (`self.SpringArm`) (`KismetMathLibrary.VInterpTo` (`SceneComponent.RelativeLocation` (`self.SpringArm`)) (`KismetMathLibrary.MakeVector` -4.64904 (+ 0.0 -4.0 (* (* _returnvalue_yaw -6.0 -0.03) -30.0 (/ (`self.CurrentSpeed`) (`self.MaxSpeed`)))) 11.933249) (`GameplayStatics.GetWorldDeltaSeconds`) 1.0) true false))

(event `InputAxis|Yaw`
  (params (AxisValue :type "Float (single-precision)"))
  ;[1 1 1] Yaw and Pitch
  (if (`self.PlayerInput`)
    (if (`self.Gravity`)
      (if (!= AxisValue 0.0)
        (`self.K2_AddActorLocalRotation` (`KismetMathLibrary.MakeRotator` AxisValue 0.0 AxisValue))))))

(event `Line trace safety`
  (bind _returnvalue (`GameplayStatics.GetWorldDeltaSeconds`))
  (bind _returnvalue_2 (`self.K2_GetActorRotation`))
  (bind _cube (`self.Cube`))
  (bind _returnvalue_3 (`SceneComponent.K2_GetComponentLocation` _cube))
  (bind (_returnvalue_roll _returnvalue_pitch) (`KismetMathLibrary.BreakRotator` (`KismetMathLibrary.RInterpTo` _returnvalue_2 (`KismetMathLibrary.MakeRotator` 0.0) _returnvalue 6.0)))
  ;[1 1 1] Track Hover and Alignment
  (if (`self.Gravity`)
    (bind (_outhit _returnvalue_4) (`KismetSystemLibrary.SphereTraceSingle` :`Start` _returnvalue_3 :`End` (+ (* (`SceneComponent.GetUpVector` _cube) -400.0) _returnvalue_3) :`Radius` 60.0 :`TraceChannel` "TraceTypeQuery1" :`DrawDebugType` "ForOneFrame"))
    (if _returnvalue_4
      (bind (_bblockinghit _binitialoverlap _time _distance _location _impactpoint _normal _impactnormal) (`GameplayStatics.BreakHitResult` _outhit))
      (`self.K2_SetActorRotation` (`KismetMathLibrary.RInterpTo` (`self.K2_GetActorRotation`) (`KismetMathLibrary.MakeRotFromZX` _impactnormal (`self.GetActorForwardVector`)) _returnvalue 6.0))
      (`self.K2_SetActorLocation` (+ _impactpoint (* _impactnormal 280.0)))
      (`/Engine/EditorBlueprintResources/StandardMacros.DoOnce` true :!label _label
        (:`Completed`
          (`PlayerController.ClientStartCameraShake` :`self` (`GameplayStatics.GetPlayerController` 0) :`Shake` "/Script/Engine.CameraShake" :`Scale` 0.7)))
      (else
        (`self.K2_AddActorWorldOffset` (0.0 0.0 -60.0))
        (`self.K2_SetActorRotation` (`KismetMathLibrary.MakeRotator` _returnvalue_roll _returnvalue_pitch (.yaw _returnvalue_2)))
        (goto _label :!via `Reset`)))))

(fn `RespawnCheck`
  (returns (PlayerIsStuck :type Boolean))
  ;[1 1 1] Checks to see if player is not moving and upside down
  (if (and (< (`KismetMathLibrary.Dot_VectorVector` (`self.GetActorUpVector`) (0.0 0.0 1.0)) 0.5) (< (`self.CurrentSpeed`) 0.5))
    (set `self.Stuck?` true)
    (else
      (set `self.Stuck?` false)))
  (return (`self.Stuck?`)))

(fn `Split_Axis`
  (params (Value :type "Float (double-precision)"))
  (returns (Pos :type "Float (double-precision)") (Neg :type "Float (double-precision)"))
  (return (`KismetMathLibrary.FClamp` Value) (`KismetMathLibrary.FClamp` (- 0.0 Value))))

(fn `UserConstructionScript`)